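; Enemy character for a necromancy game, in melee, sword or caster variants, that fights under AI and can be revived as the player's ally.
; Construction picks the attack montage per type; sphere traces or a spawned projectile deliver damage tagged with allegiance.
; ACCombatComponent handles damage, animations and cooldown events, while the Blueprint updates blackboard target and state.
; Revive plays a montage, recolors the mesh, flips it friendly and restores collision and health.
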(event `self.ReceiveBeginPlay`
  (bind _ac_combatcomponent (`self.AC_CombatComponent`))
  ;[0.007843 0.007843 0.007843] Setup functions
  (add `/Game/Necromancy/Blueprints/Player/AC_CombatComponent.CanBeDamagedAgain` _ac_combatcomponent (delegate `CanBeDamagedAgain_Event_0`))
  (add `/Game/Necromancy/Blueprints/Player/AC_CombatComponent.CanAttackAgain` _ac_combatcomponent (delegate `CanAttackAgain_Event`))
  (bind _asbp_third_person_character (cast `/Game/Necromancy/Blueprints/Player/BP_ThirdPersonCharacter` (`GameplayStatics.GetPlayerCharacter` 0)))
  (`BlackboardComponent.SetValueAsObject` (`AIBlueprintHelperLibrary.GetBlackboard` null) "Player" _asbp_third_person_character)
  (`BlackboardComponent.SetValueAsEnum` (`AIBlueprintHelperLibrary.GetBlackboard` null) "EnemyType" (`self.EnemyType`)))

(event `CanBeDamagedAgain_Event_0`
  (params (Revivable :type Boolean))
  ;[0.007843 0.007843 0.007843] Setup functions
  (set `self.CanBeDamaged` true)
  (set `self.Revivable` Revivable))

(event `CanAttackAgain_Event`
  ;[0.007843 0.007843 0.007843] Setup functions
  (set `self.CanAttack` true))

(event `/Game/Necromancy/Blueprints/Player/BPI_Damage.Damage`
  (params (DamageAmount :type "Float (double-precision)") (Friendly :type Boolean) (Damager :type "Actor Object Reference"))
  ;[0.007843 0.007843 0.007843] Take damage
  (if (`self.CanBeDamaged`)
    (if (not (== Friendly (`self.Friendly`)))
      (set `self.CanBeDamaged` false)
      (`BlackboardComponent.SetValueAsObject` (`AIBlueprintHelperLibrary.GetBlackboard` null) "Target" Damager)
      (`AIController.K2_SetFocus` (`AIBlueprintHelperLibrary.GetAIController` self) Damager)
      (bind (_newhealth _isdead) (`/Game/Necromancy/Blueprints/Player/AC_CombatComponent.DamageCalculator` (`self.AC_CombatComponent`) (`self.Health`) DamageAmount (`self.Mesh`) "/Game/Necromancy/Assets/Animations/AM_TakeDamage.AM_TakeDamage" "/Game/Necromancy/Assets/Animations/AM_Death.AM_Death"))
      (set `self.Health` _newhealth)
      (bind _output_get (set `self.IsDead` _isdead))
      (if _output_get
        (`BlackboardComponent.SetValueAsEnum` (`AIBlueprintHelperLibrary.GetBlackboard` null) "EnemyState" (enumliteral `/Game/Necromancy/Blueprints/Enemy/E_EnemyState` "NewEnumerator2"))
        (`AIController.K2_ClearFocus` (`AIBlueprintHelperLibrary.GetAIController` self))
        (`PrimitiveComponent.SetCollisionEnabled` (`self.CapsuleComponent`) "NoCollision")))))

(event `EnemyAttack`
  (bind _returnvalue (`AIBlueprintHelperLibrary.GetBlackboard` null))
  ;[0.007843 0.007843 0.007843] Attack
  (bind _isdead (message `/Game/Necromancy/Blueprints/Enemy/BPI_Communicate.CheckStatus` (`BlackboardComponent.GetValueAsObject` (`AIBlueprintHelperLibrary.GetBlackboard` null) "Target")))
  (if _isdead
    (bind (_isdead_2 _friendly) (message `/Game/Necromancy/Blueprints/Enemy/BPI_Communicate.CheckStatus` (`BlackboardComponent.GetValueAsObject` _returnvalue "Target") :!label _label))
    (if (or _isdead_2 (== _friendly (`self.Friendly`)))
      (`BlackboardComponent.SetValueAsObject` _returnvalue "Target" null)
      (`AIController.K2_ClearFocus` (`AIBlueprintHelperLibrary.GetAIController` self)))
    (elif (`self.CanAttack`)
      (set `self.CanAttack` false)
      (`/Game/Necromancy/Blueprints/Player/AC_CombatComponent.AtttackAnim` (`self.AC_CombatComponent`) (`self.Mesh`) (`self.AttackMontage`))
      (goto _label))))

(event `/Game/Necromancy/Blueprints/Enemy/BPI_Communicate.Revive`
  (bind _returnvalue (`AIBlueprintHelperLibrary.GetBlackboard` null))
  ;[0.007843 0.007843 0.007843] Revive
  (if (and (`self.IsDead`) (`self.Revivable`))
    (set `self.IsDead` false)
    (set `self.Friendly` true)
    (`|PlayMontage` (`self.Mesh`) "/Game/Necromancy/Assets/Animations/AM_Revive.AM_Revive"
      (:`then`
        (bind (_direction _newtrack_2) (`Timeline|ColorChanger` :!via `PlayFromStart`)
          (:`Update`
            (bind (_r _g _b) (`KismetMathLibrary.BreakColor` _newtrack_2))
            (`MeshComponent.SetVectorParameterValueOnMaterials` (`self.Mesh`) "Color" (`KismetMathLibrary.MakeVector` _r 0.0 _b)))))
      (:`OnCompleted`
        (`PrimitiveComponent.SetCollisionEnabled` (`self.CapsuleComponent`) "QueryAndPhysics")
        (`BlackboardComponent.SetValueAsEnum` _returnvalue "EnemyState" (enumliteral `/Game/Necromancy/Blueprints/Enemy/E_EnemyState` "NewEnumerator1"))
        (`BlackboardComponent.SetValueAsObject` _returnvalue "Target" null)
        (set `self.Health` 100.0)))))

(fn `CheckStatus`
  (returns (IsDead :type Boolean) (Friendly :type Boolean))
  (return (`self.IsDead`) (`self.Friendly`)))

(fn `EnemyKickTrace`
  (bind _mesh (`self.Mesh`))
  (bind _outhits (`KismetSystemLibrary.SphereTraceMultiForObjects` (`SceneComponent.GetSocketLocation` _mesh "foot_r") (`SceneComponent.GetSocketLocation` _mesh "foot_r") 25.0 (`|MakeArray` "ObjectTypeQuery3" :!type "EObjectTypeQuery Enum")))
  (for _array_element _outhits
    (message `/Game/Necromancy/Blueprints/Player/BPI_Damage.Damage` (`.HitActor` (`GameplayStatics.BreakHitResult` _array_element)) (`self.EnemyDamage`) (`self.Friendly`) self)))

(fn `EnemyProjectile`
  (`|SpawnActorFromClass` "/Game/Necromancy/Blueprints/BP_Projectile.BP_Projectile_C" (`SceneComponent.K2_GetComponentToWorld` (`self.ProjectileSpawn`)) "Undefined" "MultiplyWithRoot" null (`self.Friendly`) self null))

(fn `EnemySwordAttackTrace`
  (bind _sword (`self.Sword`))
  (bind _outhits (`KismetSystemLibrary.SphereTraceMultiForObjects` (`SceneComponent.GetSocketLocation` _sword "Start") (`SceneComponent.GetSocketLocation` _sword "End") 25.0 (`|MakeArray` "ObjectTypeQuery3" :!type "EObjectTypeQuery Enum")))
  (for _array_element _outhits
    (message `/Game/Necromancy/Blueprints/Player/BPI_Damage.Damage` (`.HitActor` (`GameplayStatics.BreakHitResult` _array_element)) (`self.EnemyDamage`) (`self.Friendly`) self)))

(fn `UserConstructionScript`
  (set `self.AttackMontage` (select `/Game/Necromancy/Blueprints/Enemy/E_EnemyType` (`self.EnemyType`) :`NewEnumerator0` "/Game/Necromancy/Assets/Animations/AM_Kick.AM_Kick" :`NewEnumerator1` "/Game/Necromancy/Assets/Animations/AM_EnemySwordAttack.AM_EnemySwordAttack" :`NewEnumerator2` "/Game/Necromancy/Assets/Animations/AM_EnemyCast.AM_EnemyCast" :!type "AnimMontage Object Reference"))
  (if (`|EnumEquality` (`self.EnemyType`) "NewEnumerator1")
    (`SceneComponent.SetVisibility` (`self.Sword`) true false)))