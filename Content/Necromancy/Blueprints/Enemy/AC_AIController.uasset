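; AI controller for BP_Enemy pawns that runs the melee enemy behavior tree and handles target detection.
; BeginPlay starts BT_MeleeEnemy and caches the controlled enemy.
; When AI perception updates and the blackboard has no valid Target, it checks each updated actor's status through CheckStatusMessage.
; Living actors of opposite Friendly allegiance become focus and Target while the enemy is alive, so the last match wins.
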(event `self.ReceiveBeginPlay`
  (`self.RunBehaviorTree` "/Game/Necromancy/Blueprints/Enemy/BT_MeleeEnemy.BT_MeleeEnemy")
  (bind _asbp_enemy (cast `/Game/Necromancy/Blueprints/Enemy/BP_Enemy` (`self.K2_GetPawn`)))
  (set `self.EnemyPawn` _asbp_enemy))

(event `self.AIPerception.OnPerceptionUpdated`
  (params (UpdatedActors :type "Array of Actor Object Reference (by ref)"))
  ;[0.007843 0.007843 0.007843] Detect enemy
  (`/Engine/EditorBlueprintResources/StandardMacros.IsValid` (`BlackboardComponent.GetValueAsObject` (`AIBlueprintHelperLibrary.GetBlackboard` null) "Target")
    (:`Is Not Valid`
      (for _array_element UpdatedActors
        (bind (_isdead _friendly) (message `/Game/Necromancy/Blueprints/Enemy/BPI_Communicate.CheckStatus` _array_element))
        (if (and (not _isdead) (not (== _friendly (`/Game/Necromancy/Blueprints/Enemy/BP_Enemy.Friendly` (`self.EnemyPawn`)))) (not (`/Game/Necromancy/Blueprints/Enemy/BP_Enemy.IsDead` (`self.EnemyPawn`))))
          (`self.K2_SetFocus` _array_element)
          (`BlackboardComponent.SetValueAsObject` (`AIBlueprintHelperLibrary.GetBlackboard` null) "Target" _array_element))))))

(fn `UserConstructionScript`)