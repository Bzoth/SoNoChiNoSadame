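; Actor component for combat that resolves damage and plays attack, hit and death montages on a supplied skeletal mesh.
; DamageCalculator subtracts damage from the passed-in health, triggers the hit or death animation, and returns new health and a death flag.
; Dispatchers signal when attacking or taking damage is allowed again: on montage completion, after a short random delay if interrupted, or a fixed delay after death starts.
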(event `DeathAnim`
  (params (SkeletalMesh :type "SkeletalMeshComponent Object Reference") (Montage :type "AnimMontage Object Reference"))
  ;[0.007843 0.007843 0.007843] Death
  (`|PlayMontage` SkeletalMesh Montage
    (:`then`
      (`KismetSystemLibrary.Delay` 3.0)
      (`self.CanBeDamagedAgain` true))))

(event `TakeDamageAnim`
  (params (SkeletalMesh :type "SkeletalMeshComponent Object Reference") (Montage :type "AnimMontage Object Reference"))
  ;[0.007843 0.007843 0.007843] Take damage
  (`|PlayMontage` SkeletalMesh Montage
    (:`OnCompleted`
      _)
    (:`OnInterrupted`
      (`KismetSystemLibrary.Delay` (`KismetMathLibrary.RandomFloatInRange` 0.5 1.0))))
  (`self.CanBeDamagedAgain` false))

(event `AtttackAnim`
  (params (SkeletalMesh :type "SkeletalMeshComponent Object Reference") (Montage :type "AnimMontage Object Reference"))
  ;[0.007843 0.007843 0.007843] Attack
  (`|PlayMontage` SkeletalMesh Montage
    (:`OnCompleted`
      _)
    (:`OnInterrupted`
      (`KismetSystemLibrary.Delay` (`KismetMathLibrary.RandomFloatInRange` 0.5 1.0))))
  (`self.CanAttackAgain`))

(fn `DamageCalculator`
  (params (Health :type "Float (double-precision)") (Damage :type "Float (double-precision)") (SkeletalMesh :type "SkeletalMeshComponent Object Reference") (TakeDamageMontage :type "AnimMontage Object Reference") (DeathMontage :type "AnimMontage Object Reference"))
  (returns (NewHealth :type "Float (double-precision)") (IsDead :type Boolean))
  (bind _returnvalue (- Health Damage))
  (if (<= _returnvalue 0.0)
    (`self.DeathAnim` (`local.SkeletalMesh`) (`local.DeathMontage`))
    (return 0.0 true)
    (else
      (`self.TakeDamageAnim` (`local.SkeletalMesh`) (`local.TakeDamageMontage`))
      (return _returnvalue false))))